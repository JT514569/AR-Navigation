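; Map segment actor for AR navigation that pairs a map image plane with a minimap mesh for one section or floor.
; The construction script applies the material, mesh, scale and offset to its components.
; BeginPlay hides the plane in game and, after a brief delay, shifts the minimap mesh by a mapping offset.
; With floor auto-detection on, Tick shows that mesh only while the camera's Z lies within the segment's height range.
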(event Custom|SetupMinimap
  (bind _segmentmeshminimapcomponent (Variables|Default|GetSegmentMeshMinimapComponent))
  ;[1 1 1] Minimap Setup
  (Transformation|SetWorldLocation _segmentmeshminimapcomponent (+ (Transformation|GetWorldLocation _segmentmeshminimapcomponent) (Variables|Segment|GetminimapMappingOffset)) false false))

(event EventBeginPlay
  (bind _segmentmeshminimapcomponent (Variables|Default|GetSegmentMeshMinimapComponent))
  ;[1 1 1] Begin Play
  (Development|SetHiddeninGame (Variables|Default|GetSegmentMapPlane) true false)
  ;[1 1 1] Minimap Setup
  (Utilities|FlowControl|Delay 0.02)
  (Transformation|SetWorldLocation _segmentmeshminimapcomponent (+ (Transformation|GetWorldLocation _segmentmeshminimapcomponent) (Variables|Segment|GetminimapMappingOffset)) false false))

(event EventTick
  (params (DeltaSeconds :type Float%20%28single-precision%29))
  (bind _segmentcomponent (Variables|Default|GetSegmentComponent))
  (bind _returnvalue (Transformation|GetWorldLocation _segmentcomponent))
  (bind _z (Math|Vector|BreakVector _returnvalue))
  ;[1 1 1] Detect Floor
  (if (Variables|Floor|GetautoDetectFloor)
    (Rendering|SetVisibility (Variables|Default|GetSegmentMeshMinimapComponent) (Math|Float|InRange(Float) (.Z (Math|Vector|BreakVector (Transformation|GetWorldLocation (Variables|/Script/Engine.PlayerCameraManager|GetTransformComponent (Game|GetPlayerCameraManager 0))))) _z (+ _z (* (Variables|Segment|GetsegmentHeigh) 1e+02))) false)))

(fn ConstructionScript
  (bind _segmentmapplane (Variables|Default|GetSegmentMapPlane))
  (bind _segmentscale (Variables|Segment|GetsegmentScale))
  (bind _segmentoffset (Variables|Segment|GetsegmentOffset))
  (bind (_x _y) (Math|Vector2D|BreakVector2D _segmentoffset))
  (Transformation|SetRelativeScale3D _segmentmapplane (Math|Conversions|ToVector(Float) (Variables|Segment|GetsegmentMapScale)))
  (Rendering|Material|SetMaterial _segmentmapplane 0 (Variables|Segment|GetsegmentMapMaterial))
  (Components|StaticMesh|SetStaticMesh (Variables|Default|GetSegmentMeshMinimapComponent) (Variables|Segment|GetsegmentMesh))
  (Transformation|SetRelativeTransform (Variables|Default|GetSegmentComponent) (Math|Transform|MakeTransform (Math|Vector|MakeVector _x _y 0.0) "0, 0, 0" (Math|Vector|MakeVector _segmentscale _segmentscale (Variables|Segment|GetsegmentHeigh))) false false))
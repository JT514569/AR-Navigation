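; Minimap actor in AR navigation, named as the 2D map image provider; no capture logic appears in its graphs.
; Each Tick sets the root's world transform from MakeTransform, without sweep or teleport.
; The MakeTransform graph holds a calculation placing the actor high above the player camera, following its yaw with a quarter-turn offset, though that node appears unconnected.
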(event EventTick
  (params (DeltaSeconds :type Float%20%28single-precision%29))
  (Transformation|SetWorldTransform (Variables|Default|GetDefaultSceneRoot) (Math|Transform|MakeTransform) false false))

(fn ConstructionScript)
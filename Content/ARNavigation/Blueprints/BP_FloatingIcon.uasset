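; BP_FloatingIcon is an AR navigation actor that displays a pulsing icon with text labels.
; On BeginPlay, a timeline subtly scales the root, creating the animation.
; It creates left and right text widgets for its two widget components and copies its Text into both.
; It also applies IconMaterial to element 1 of both the Icon and IconFlipped components.
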(event EventBeginPlay
  (Utilities|FlowControl|Sequence
    (:then_0
      (|AnimateMovement))
    (:then_1
      (bind (_widget _widget1) (UserInterface|CreateWidget))
      (Rendering|Material|SetMaterial)
      (Rendering|Components|TextRender|SetText _widget _widget1))))

(fn ConstructionScript)
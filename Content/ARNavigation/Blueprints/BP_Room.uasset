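; BP_Room is a room actor in the AR navigation project that represents a room's bounds with a cube, hidden at BeginPlay.
; A non-zero Size, combined with Height, scales the cube in the construction script.
; With Size left at zero, BeginPlay uses four world-axis line traces to the surrounding geometry to center and scale it automatically.
; CompareInRange tests whether a value lies within a scaled extent around a coordinate.
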(event EventBeginPlay
  (Rendering|SetVisibility (Variables|Default|GetCube) false false)
  (bind (_location _distance) (CallFunction|LineTrace "-9999.000000, 0, 0"))
  (bind (_location_2 _distance_2) (CallFunction|LineTrace "9999.000000, 0, 0"))
  (bind (_location_3 _distance_3) (CallFunction|LineTrace "0,-9999.000000, 0"))
  (bind (_location_4 _distance_4) (CallFunction|LineTrace "0,9999.000000, 0"))
  (Math|Transform|MakeTransform (|CalculateLocation _location_2 _location _location_4 _location_3) (|CalculateScale _distance_2 _distance _distance_4 _distance_3)))

(fn ConstructionScript
  (bind _size (Variables|Room|GetSize))
  (bind (_x _y) (Math|Vector2D|BreakVector2D _size))
  (Rendering|Material|SetMaterial (Variables|Default|GetCube) 0 (Variables|Room|GetdebugMaterial))
  (if (not (Math|Vector|Equal(Vector) :A (Variables|Room|GetSize)))
    (Transformation|SetWorldScale3D (Variables|Default|GetCube) (Math|Vector|MakeVector _x _y (Variables|Room|GetHeight)))))

(fn CompareinRange
  (params (Value :type Float%20%28single-precision%29) (XYZ :type Float%20%28single-precision%29) (SCALE :type Float%20%28single-precision%29))
  (bind _returnvalue (* SCALE 5e+01))
  (return (Math|Float|InRange(Float) Value (- XYZ _returnvalue) (+ XYZ _returnvalue))))

(fn LineTrace
  (params (Offset :type Vector))
  (bind _defaultsceneroot (Variables|Default|GetDefaultSceneRoot))
  (bind _returnvalue (Transformation|GetWorldLocation _defaultsceneroot))
  (bind (_outhit _returnvalue_2) (Collision|LineTraceByChannel _returnvalue (+ _returnvalue Offset) "TraceTypeQuery1" true 0 "None" true "(R=0.103405,G=1.000000,B=0.000000,A=1.000000)" "(R=1.000000,G=0.000000,B=0.103829,A=1.000000)" 8888.0))
  (if _returnvalue_2
    (return (.ImpactPoint (Collision|BreakHitResult _outhit)) (.Distance (Collision|BreakHitResult _outhit)))))
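; AR navigation marker actor that displays a WB_Marker widget and tracks when the user is close.
; ConfigureWidget builds the widget and caches WB_MainUI; HideMarker hides the scene and stops proximity checks.
; Tick sets widget rotation through MakeRotation, intended to face the camera by yaw.
; Paired DoOnce nodes reset each other, so MainUI adds or removes the marker only on crossing the distance threshold.
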(event Custom|ConfigureWidget
  ;[1 1 1] Create Marker
  (bind _returnvalue (UserInterface|CreateWidget "/Game/ARNavigation/Blueprints/UI/Marker/WB_Marker.WB_Marker_C" (Game|GetPlayerController 0)))
  (Variables|/Game/ARNavigation/Blueprints/UI/Marker/WB_Marker.WB_Marker_C|SetBP_Placeable _returnvalue self)
  (Variables|/Game/ARNavigation/Blueprints/UI/Marker/WB_Marker.WB_Marker_C|SetcustomMarker _returnvalue (Variables|Default|GetcustomMarker))
  (UserInterface|SetWidget (Variables|Default|GetWidget) _returnvalue)
  (bind _foundwidgets (Widget|GetAllWidgetsOfClass "/Game/ARNavigation/Blueprints/UI/MainUI/WB_MainUI.WB_MainUI_C" true))
  (Variables|Default|SetmainUI (Utilities|Array|Get(acopy) _foundwidgets)))

(event Custom|HideMarker
  ;[1 1 1] Hide Marker
  (Rendering|SetVisibility (Variables|Default|GetScene) false true)
  (Variables|Default|SetisHidden true))

(event EventTick
  (params (DeltaSeconds :type Float%20%28single-precision%29))
  (bind _self self)
  (bind _mainui (Variables|Default|GetmainUI))
  ;[1 1 1] Rotate Marker to the user
  (Transformation|SetWorldRotation (Variables|Default|GetWidget) (|MakeRotation) false false)
  ;[1 1 1] Check if the user is close
  (if (not (Variables|Default|GetisHidden))
    (if (<= (Transformation|GetDistanceTo (Game|GetPlayerCameraManager 0) self) 1e+02)
      (Utilities|FlowControl|Sequence
        (:then_0
          (Utilities|FlowControl|DoOnce false :!label _label
            (:Completed
              (Default|AddNearMarker _mainui _self))))
        (:then_1
          (goto _label_2 Reset)))
      (else
        (Utilities|FlowControl|Sequence
          (:then_0
            (Utilities|FlowControl|DoOnce false :!label _label_2
              (:Completed
                (Default|RemoveNearMarker _mainui _self))))
          (:then_1
            (goto _label Reset)))))))

(fn ConstructionScript)
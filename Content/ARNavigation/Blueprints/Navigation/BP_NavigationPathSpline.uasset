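; BP_NavigationPathSpline draws an AR navigation path by spawning arrow actors at regular intervals along its spline.
; UpdateDrawPath derives a count from the spline length and a Spacing value, then loops to read world location and rotation at each step's distance along the spline.
; AddArrow spawns a BP_Arrow at each point, flagging it as non-minimap and passing it the navigation actor and its distance.
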(event Custom|UpdateDrawPath
  (bind _index (|ForLoop (|GetRemainder))
    (:LoopBody
      (|AddArrow (.Location (|GetTransform _index)) (.Rotation (|GetTransform _index)) (.Distance (|GetTransform _index))))))

(fn ConstructionScript)
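; BP_Arrow is an AR navigation marker that animates an arrow and its shadow along the Navigation spline.
; On BeginPlay, a timeline drives updates that pass its value to GetTransformAlongSpline, whose nodes sample world location and rotation at Distance minus that value.
; The resulting transform positions the shadow on the path and the arrow at a fixed height above it, both at unit scale.
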(event EventBeginPlay
  (bind _value (|TimelineAnimation)
    (:Update
      (|SetArrowTransform (.Location (|GetTransformAlongSpline _value)) (.Rotation (|GetTransformAlongSpline _value)))
      (|SetShadowTransform (.Location (|GetTransformAlongSpline _value)) (.Rotation (|GetTransformAlongSpline _value))))))

(fn ConstructionScript)